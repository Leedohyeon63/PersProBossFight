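; BP_PailNail is a homing projectile that damages BP_Sinner.
; On BeginPlay it finds the BP_Sinner actor, sets its root component as the PailNail component's homing target, then destroys itself after a one-second delay.
; That timed cleanup runs only when a Sinner is found.
; Overlapping a BP_Sinner applies damage and destroys the nail immediately, while other actors are ignored.
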(event `self.ReceiveBeginPlay`
  (bind _returnvalue (`GameplayStatics.GetActorOfClass` "/Game/Sinner/BossAI/BP_Sinner.BP_Sinner_C"))
  (`/Engine/EditorBlueprintResources/StandardMacros.IsValid` _returnvalue
    (:`Is Valid`
      (set `ProjectileMovementComponent.HomingTargetComponent` (`Actor.RootComponent` _returnvalue) (`self.PailNail`))
      (`KismetSystemLibrary.Delay` 1.0)
      (`self.K2_DestroyActor`))))

(event `self.ReceiveActorBeginOverlap`
  (params (OtherActor :type "Actor Object Reference"))
  (bind _asbp_sinner (cast `/Game/Sinner/BossAI/BP_Sinner` OtherActor))
  (`GameplayStatics.ApplyDamage` _asbp_sinner (`self.Damge`))
  (`self.K2_DestroyActor`))

(fn `UserConstructionScript`)